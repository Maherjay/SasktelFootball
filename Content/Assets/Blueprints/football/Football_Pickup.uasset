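; Football_Pickup is a grabbable football actor that VR motion controllers can pick up and throw.
; Pickup turns off physics and snaps the ball to the controller's FootballSocket with a fixed grip rotation.
; Drop re-enables physics, detaches the ball and sets an angular velocity to make it spiral.
; Five seconds after release it freezes and teleports back to a hard-coded start position and rotation.
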(event EventBeginPlay)

(event Collision|EventActorBeginOverlap
  (params (OtherActor :type Actor%20Object%20Reference)))

(event EventTick
  (params (DeltaSeconds :type Float%20%28single-precision%29)))

(event EventPickup
  (params (AttachTo :type Scene%20Component%20Object%20Reference))
  (Physics|SetSimulatePhysics (Variables|Debug|GetStaticMeshComponent) false)
  (Transformation|AttachComponentToComponent self AttachTo "FootballSocket" "SnapToTarget" "SnapToTarget" "KeepWorld" false)
  (Transformation|SetRelativeRotation (Variables|Debug|GetStaticMeshComponent) "110.000000, 0, 0" false false))

(event EventDrop
  (bind _staticmeshcomponent (Variables|Debug|GetStaticMeshComponent))
  (Physics|SetSimulatePhysics (Variables|Debug|GetStaticMeshComponent) true)
  (Transformation|DetachFromActor "KeepWorld" "KeepWorld" "KeepWorld")
  ;[1 1 1] Adding rotation to make ball spiral
  (Class|PrimitiveComponent|SetPhysicsAngularVelocityinDegrees (Variables|Debug|GetStaticMeshComponent) "0,15.000000, 0" false "None")
  ;[1 1 1] Reset ball
  (Utilities|FlowControl|Delay 5.0)
  (Physics|SetSimulatePhysics _staticmeshcomponent false)
  (Transformation|SetWorldLocation _staticmeshcomponent "10.000000,-60.000000,110.000000" false true)
  (Transformation|SetWorldRotation _staticmeshcomponent "0, 0, 0" false false))

(fn ConstructionScript)